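; BP_PlayerCharacter is the player character Blueprint, handling HUD setup and health-change debug output.
; On BeginPlay it creates the crosshair and player health widgets and adds both to the viewport.
; It binds to the attribute component's OnHealthChanged event and prints the delta and new health as debug text.
; Tick and the construction script are empty, and a leftover health print is never executed.
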(event OnHealthChanged(AttributeComp)
  (params (InstigatorActor :type Actor%20Object%20Reference) (OwningComp :type R%20Attribute%20Component%20Object%20Reference) (NewHealth :type Float%20%28single-precision%29) (Delta :type Float%20%28single-precision%29))
  (Development|PrintText (Utilities|Text|FormatText "Delata: {d} New: {n}" Delta NewHealth)))

(event EventBeginPlay
  (bind _returnvalue (UserInterface|CreateWidget "/Game/ActionRouglike/UI/WBP_Croshair.WBP_Croshair_C"))
  (UserInterface|Viewport|AddtoViewport _returnvalue 0)
  (bind _returnvalue_2 (UserInterface|CreateWidget "/Game/ActionRouglike/UI/WBP_PlayerHealth.WBP_PlayerHealth_C"))
  (UserInterface|Viewport|AddtoViewport _returnvalue_2 0))

(event Collision|EventActorBeginOverlap
  (params (OtherActor :type Actor%20Object%20Reference)))

(event EventTick
  (params (DeltaSeconds :type Float%20%28single-precision%29)))

(fn ConstructionScript)
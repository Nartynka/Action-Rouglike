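; BP_ProjectileCannon is a turret actor that spawns a BP_MagicProjectile every two seconds on a looping timer started at BeginPlay.
; Each tick it rotates its Arrow component to face the first player's pawn using a look-at rotation.
; Projectiles spawn with the actor's transform rather than the Arrow's, so their aim follows the Arrow only if it is the root component.
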(event Custom|SpawnProjecitle
  (Game|SpawnActorfromClass "/Game/ActionRouglike/BP_MagicProjectile.BP_MagicProjectile_C" (Transformation|GetActorTransform) "Undefined" "MultiplyWithRoot" 0 0))

(event EventBeginPlay
  (Utilities|Time|SetTimerbyEvent (delegate Custom|SpawnProjecitle) 2.0 true))

(event EventTick
  (params (DeltaSeconds :type Float%20%28single-precision%29))
  (Transformation|SetWorldRotation (Variables|Default|GetArrow) (Math|Rotator|FindLookatRotation (Transformation|GetActorLocation) (Transformation|GetActorLocation (Game|Player|GetPlayerPawn 0))) false false))

(fn ConstructionScript)